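; Temporary Stage 3 trigger that starts a boss encounter on its first overlap by any actor.
; It finds the BossEncounterManager, resets it, binds to its boss's phase-started event, then starts the encounter with the player character, printing debug results.
; A phase handler teleports the boss to the manager's location for combat phases 2 and 3.
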(event `self.ReceiveActorBeginOverlap`
  (params (OtherActor :type "Actor Object Reference"))
  (bind _currentbossencountermanager (`self.CurrentBossEncounterManager`))
  (bind _currentboss (`BossEncounterManager.CurrentBoss` _currentbossencountermanager))
  (if (not (`self.bTriggered`))
    (set `self.bTriggered` true)
    (bind _returnvalue (`GameplayStatics.GetActorOfClass` "/Script/MyNiceLittleCat.BossEncounterManager"))
    (bind _output_get (set `self.CurrentBossEncounterManager` _returnvalue))
    (`BossEncounterManager.ResetEncounter` _output_get)
    (`/Engine/EditorBlueprintResources/StandardMacros.IsValid` _currentbossencountermanager
      (:`Is Valid`
        (add `BossCharacter.OnPhaseStarted` _currentboss (`|CreateDelegate` :!event `TeleportBossPerPhase`))
        (`KismetSystemLibrary.PrintString` (`KismetSystemLibrary.GetObjectName` _currentboss))
        (bind _asplayer_character (cast `PlayerCharacter` (`GameplayStatics.GetPlayerCharacter` 0)))
        (bind _returnvalue_2 (`BossEncounterManager.StartEncounter` (`self.CurrentBossEncounterManager`) _asplayer_character))
        (if _returnvalue_2
          (`KismetSystemLibrary.PrintString` "Success to Start Encounter")
          (else
            (`KismetSystemLibrary.PrintString` "Failed to Start Encounter")))))))

(event `TeleportBossPerPhase`
  (params (Boss :type "BossCharacter Object Reference") (EndedPhaseId :type Name))
  (switch `name` EndedPhaseId
    (:`CombatPhase2`
      (`self.K2_SetActorLocation` Boss (`self.K2_GetActorLocation` (`self.CurrentBossEncounterManager`)) false true))
    (:`CombatPhase3`
      (`self.K2_SetActorLocation` Boss (`self.K2_GetActorLocation` (`self.CurrentBossEncounterManager`)) false true))))

(fn `UserConstructionScript`)