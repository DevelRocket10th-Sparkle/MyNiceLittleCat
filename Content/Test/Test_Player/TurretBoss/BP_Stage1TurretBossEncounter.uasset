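; Encounter controller for the Stage 1 turret boss arena, driven by a fast looping ArenaCheck timer that polls the player.
; A box test on ArenaTrigger starts a Ready encounter and deactivates EntryDoor on success.
; Waiting resets the encounter and reactivates the door, while Cleared reactivates it once.
; The check also kills a player who falls below a height threshold; a reset for leaving mid-fight is present but unconnected.
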(event `self.ReceiveBeginPlay`
  (`KismetSystemLibrary.K2_SetTimer` null "ArenaCheck" 0.05 true))

(fn `ArenaCheck`
  (bind _encounterstate (`self.EncounterState`))
  (bind _arenatrigger (`self.ArenaTrigger`))
  (bind _asplayer_character (cast `PlayerCharacter` (`GameplayStatics.GetPlayerCharacter` 0))
    (:`then`
      (if (< (.z (`self.K2_GetActorLocation` _asplayer_character)) -50.0)
        (`PlayerCharacter.ApplyPlayerHit` _asplayer_character 99999.0 (0.0 0.0 0.0))))
    (:`CastFailed`
      _))
  (if (`|EnumEquality` _encounterstate "Ready")
    (bind _asplayer_character_2 (cast `PlayerCharacter` (`GameplayStatics.GetPlayerCharacter` 0)))
    (if (`KismetMathLibrary.IsPointInBox` (`self.K2_GetActorLocation` _asplayer_character_2) (`SceneComponent.K2_GetComponentLocation` _arenatrigger) (`BoxComponent.GetScaledBoxExtent` _arenatrigger))
      (bind _returnvalue (`self.StartEncounter` _asplayer_character_2))
      (if _returnvalue
        (`GimmickActorBase.SetActivated` (`self.EntryDoor`) false null)))
    (elif (`|EnumEquality` _encounterstate "Waiting")
      (`self.ResetEncounter`)
      (`GimmickActorBase.SetActivated` (`self.EntryDoor`) true null)
      (elif (`|EnumEquality` _encounterstate "Cleared")
        (if (not (`self.bClearHandled`))
          (set `self.bClearHandled` true)
          (`GimmickActorBase.SetActivated` (`self.EntryDoor`) true null))))))

(fn `UserConstructionScript`)