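; Stage 2 gimmick cinematic actor that plays a skippable reveal sequence the first time its receiver is activated.
; The sequence uses the actor's transform as origin, and its reveal marker activates RevealTargets such as lamps and doors.
; Player input, enemies, pet Reflect mode and cursor are suspended until playback ends or fails.
; Repeat or startup (save-restore) activations, missing sequences and playback failures activate targets directly; deactivation switches them off.
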(event `self.ReceiveBeginPlay`
  ;[0.35 0.55 1 1 24] ① 시작 준비 — 맵 시작 0.1초 뒤 bReady = true. 그 전에 들어온 신호(세이브 복원)는 연출 없이 바로 전달
  (`KismetSystemLibrary.Delay` 0.1)
  (set `self.bReady` true))

(event `self.K2_OnActivationChanged`
  (params (bNewActivated :type Boolean) (ChangeInstigator :type "Actor Object Reference"))
  (bind _revealtargets (`self.RevealTargets`))
  ;[1 0.75 0.25 1 24] ② 수신기 신호 받음 — 꺼짐: 대상 끄기 / 켜짐: 첫 재생이면 연출(Cinematic_Play), 아니면 대상 바로 켜기
  (if bNewActivated
    (if (and (and (`self.bReady`) (not (`self.bPlayed`))) (`KismetSystemLibrary.IsValid` (`self.Sequence`)))
      (set `self.bPlayed` true)
      (`self.Cinematic_Play`)
      (else
        ;;[0.45 0.45 0.45 1 16] 조건 불충족(불러오기·재진입) → 대상 바로 켜기
        (for _array_element _revealtargets
          (message `ActivatableInterface.Activate` _array_element self))))
    (else
      ;;[0.45 0.45 0.45 1 16] 신호 꺼짐 → 대상(RevealTargets) 끄기
      (for _array_element_2 _revealtargets
        (message `ActivatableInterface.Deactivate` _array_element_2 self)))))

(event `Cinematic_Play`
  ;[0.4 0.9 0.4 1 24] ③ Cinematic_Play — 시퀀스 재생(스킵 가능) → 잠금 → Reveal 마커에서 가로등·문 켜기 → 재생이 끝나면 잠금 해제 (스킵해도 마커는 전달됨, 재생 실패 시 바로 켜고 해제)
  ;;[0.45 0.45 0.45 1 16] 시퀀스 플레이어 생성 — 이 액터를 좌표 원점으로 (레벨 인스턴스 위치 따라감)
  (bind _marker (`PlayCinematicAsyncAction.PlayCinematic` (make `CinematicRequest` (`self.Sequence`) _ true (`self.GetTransform`)))
    (:`then`
      ;;[0.45 0.45 0.45 1 16] 카메라가 비출 때 대상 켜기 → 잠시 보여준 뒤 잠금 해제
      (`self.Cinematic_Lock`))
    (:`OnMarker`
      (if (`KismetStringLibrary.EqualEqual_StrStr` (`.Label` (break `CinematicMarker` _marker)) (`self.RevealMarker`))
        (for _array_element (`self.RevealTargets`) :!label _label
          (message `ActivatableInterface.Activate` _array_element self))))
    (:`OnEnded`
      ;; 종료(완료·스킵·중단·시간 초과) → 잠금 해제
      (`self.Cinematic_Unlock`))
    (:`OnFailed`
      (`self.Cinematic_Unlock`)
      (goto _label))))

(event `Cinematic_Lock`
  (bind _returnvalue (`GameplayStatics.GetPlayerController` 0))
  ;[1 0.45 0.45 1 24] ④ Cinematic_Lock — 연출 동안 플레이어 입력·몬스터·펫 반사판·마우스 커서를 멈춤
  ;;[0.45 0.45 0.45 1 16] 입력 잠금 (컨트롤러·폰)
  (`self.DisableInput` (`GameplayStatics.GetPlayerPawn` 0) _returnvalue)
  ;;[0.45 0.45 0.45 1 16] 몬스터 정지: 시간 배율 0 (연출 중 피해 방지)
  (bind _outactors (`GameplayStatics.GetAllActorsOfClass` "/Script/MyNiceLittleCat.EnemyCharacter"))
  (for _array_element _outactors
    (set `Actor.CustomTimeDilation` 0.0 _array_element))
  ;;[0.45 0.45 0.45 1 16] 펫이 반사 모드면 기본 모드로 (반사판 프리뷰·설치 끔) → 커서 숨김
  (bind _returnvalue_2 (`GameplayStatics.GetActorOfClass` "/Script/MyNiceLittleCat.PetCharacter"))
  (set `self.bPetWasReflect` (`PetCharacter.IsModeAbilityActive` _returnvalue_2 "Reflect"))
  (if (`self.bPetWasReflect`)
    (`PetCharacter.RequestMode` _returnvalue_2 "Basic"))
  (set `PlayerController.CurrentMouseCursor` "None" _returnvalue))

(event `Cinematic_Unlock`
  (bind _returnvalue (`GameplayStatics.GetPlayerController` 0))
  ;[0.5 0.85 1 1 24] ⑤ Cinematic_Unlock — ④에서 멈춘 것을 되돌림
  ;;[0.45 0.45 0.45 1 16] 입력 잠금 해제
  (`self.EnableInput` (`GameplayStatics.GetPlayerPawn` 0) _returnvalue)
  ;;[0.45 0.45 0.45 1 16] 몬스터 재개: 시간 배율 1
  (bind _outactors (`GameplayStatics.GetAllActorsOfClass` "/Script/MyNiceLittleCat.EnemyCharacter"))
  (for _array_element _outactors
    (set `Actor.CustomTimeDilation` 1.0 _array_element))
  ;;[0.45 0.45 0.45 1 16] 반사 모드였으면 되돌림 → 커서 다시 표시
  (bind _returnvalue_2 (`GameplayStatics.GetActorOfClass` "/Script/MyNiceLittleCat.PetCharacter"))
  (if (`self.bPetWasReflect`)
    (`PetCharacter.RequestMode` _returnvalue_2 "Reflect"))
  (set `PlayerController.CurrentMouseCursor` "Default" _returnvalue))

(fn `UserConstructionScript`)